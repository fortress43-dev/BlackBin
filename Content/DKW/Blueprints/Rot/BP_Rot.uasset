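; BP_Rot is a pawn that uses AI movement to follow the player.
; It caches BP_Player on BeginPlay, then MoveAI sends it to a random reachable point in a very small radius around that player.
; MoveAI re-calls itself after a short delay on success or failure.
; Tick also calls it every frame while UsingAIMove is true, so requests come from both paths.
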(event `self.ReceiveBeginPlay`
  ;[0.7292 0 1] Init & Activation
  (bind _returnvalue (`GameplayStatics.GetActorOfClass` "/Game/CSK/Blueprints/BP_Player.BP_Player_C"))
  (set `self.Player` _returnvalue))

(event `self.ReceiveTick`
  (params (DeltaSeconds :type "Float (single-precision)"))
  ;[0.7292 0 1] Init & Activation
  (if (`self.usingAIMove`)
    (`self.MoveAI`)))

(event `MoveAI`
  ;[1 1 1] AI Move Proccess
  (bind _output_get (set `self.Random Location` (`NavigationSystemV1.K2_GetRandomReachablePointInRadius` (`self.K2_GetActorLocation` (`self.Player`)) 2.0 null null)))
  (`|AIMoveTo` self _output_get null
    (:`OnSuccess`
      (`KismetSystemLibrary.Delay` 0.2))
    (:`OnFail`
      (`KismetSystemLibrary.Delay` 0.2)))
  (`self.MoveAI`))

(fn `UserConstructionScript`)