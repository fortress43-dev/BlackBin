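; BP_AIRot is an AI pawn that follows the player by moving to random reachable points close to the player's location.
; BeginPlay caches the BP_Player actor and starts MoveAI, which issues AIMoveTo and calls itself again after a delay, shorter on failure than on success.
; Tick also feeds directly into the same move logic, so a new destination is requested every frame alongside the delayed loop.
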(event `self.ReceiveBeginPlay`
  (bind _returnvalue (`GameplayStatics.GetActorOfClass` "/Game/CSK/Blueprints/BP_Player.BP_Player_C"))
  (set `self.Player` _returnvalue)
  (`self.MoveAI`))

(event `self.ReceiveTick`
  (params (DeltaSeconds :type "Float (single-precision)"))
  (bind _output_get (set `self.Random Location` (`NavigationSystemV1.K2_GetRandomReachablePointInRadius` (`self.K2_GetActorLocation` (`self.Player`)) 10.0 null null) :!label _label))
  (`|AIMoveTo` self _output_get null
    (:`OnSuccess`
      (`KismetSystemLibrary.Delay` 2.0))
    (:`OnFail`
      (`KismetSystemLibrary.Delay` 0.2)))
  (`self.MoveAI`))

(event `MoveAI`
  (goto _label))

(fn `UserConstructionScript`)